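; Flamethrower weapon Blueprint that damages what its fire reaches, controlled by fire and stop events.
; Firing plays a timeline from the start, whose FireLen track sets the reach of a Visibility box trace along the Arrow's forward vector.
; Every timeline update applies WeaponDamage to the hit actor, credited to the owner, so damage depends on update rate.
; Stopping halts the timeline; trace debug drawing is left on.
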(event `self.BpFireEvent`
  (bind _returnvalue (`self.GetOwner`))
  (bind _arrow (`self.Arrow`))
  (bind _returnvalue_2 (`SceneComponent.K2_GetComponentLocation` _arrow))
  (bind (_direction _firelen) (`Timeline|Timeline` :!via `PlayFromStart` :!label _label)
    (:`Update`
      (bind _output_get (set `self.FireLength` _firelen))
      (bind _outhit (`KismetSystemLibrary.BoxTraceSingle` :`Start` _returnvalue_2 :`End` (+ (* (`SceneComponent.GetForwardVector` _arrow) _output_get) _returnvalue_2) :`HalfSize` (50.0 50.0 35.0) :`TraceChannel` "TraceTypeQuery1" :`DrawDebugType` "ForDuration" :`DrawTime` 0.2))
      (`GameplayStatics.ApplyDamage` (`.HitActor` (`GameplayStatics.BreakHitResult` _outhit)) (`self.WeaponDamage`) (`self.GetInstigatorController` _returnvalue) _returnvalue))))

(event `self.BpStopEvent`
  (goto _label :!via `Stop`))

(fn `UserConstructionScript`)